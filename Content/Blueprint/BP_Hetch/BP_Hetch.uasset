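; BP_Hetch is a key-locked sliding hatch that opens when the player character enters its trigger box.
; On overlap, it checks the BP_FirstPersonCharacter's KeyRing for KeyNeeded, printing a hint if the key is missing.
; A timeline lerps the Hetch component from its cached start location along negative Y to open.
; When the character leaves, an open hatch closes by reversing the same timeline.
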(event OnComponentBeginOverlap(Box)
  (params (OverlappedComponent :type Primitive%20Component%20Object%20Reference) (OtherActor :type Actor%20Object%20Reference) (OtherComp :type Primitive%20Component%20Object%20Reference) (OtherBodyIndex :type Integer) (bFromSweep :type Boolean) (SweepResult :type Hit%20Result%20Structure%20%28by%20ref%29))
  (bind _asbp_first_person_character (Utilities|Casting|CastToBP_FirstPersonCharacter OtherActor))
  (if (Utilities|Array|ContainsItem (Variables|/Game/Blueprint/BP_FirstPerson/Blueprints/BP_FirstPersonCharacter.BP_FirstPersonCharacter_C|GetKeyRing _asbp_first_person_character) (Variables|Default|GetKeyNeeded))
    (CallFunction|OpenHetch)
    (Variables|Default|SetHetchOpen? true)
    (else
      (Development|PrintString "GO FIND THE KEY!"))))

(event OnComponentEndOverlap(Box)
  (params (OverlappedComponent :type Primitive%20Component%20Object%20Reference) (OtherActor :type Actor%20Object%20Reference) (OtherComp :type Primitive%20Component%20Object%20Reference) (OtherBodyIndex :type Integer))
  (Utilities|Casting|CastToBP_FirstPersonCharacter OtherActor)
  (if (Variables|Default|GetHetchOpen?)
    (CallFunction|CloseHetch)
    (Variables|Default|SetHetchOpen? false)))

(event Custom|OpenHetch
  (bind _startposition (Variables|Default|GetStartPosition))
  (bind _speed (Timeline|Timeline Play)
    (:Update
      (Transformation|SetRelativeLocation (Variables|Default|GetHetch) (Math|Vector|Lerp(Vector) _startposition (- _startposition "0.000000,500.000000,0.000000") _speed) false false))))

(event Custom|CloseHetch
  (bind _startposition (Variables|Default|GetStartPosition))
  (bind _speed (Timeline|Timeline Reverse)
    (:Update
      (Transformation|SetRelativeLocation (Variables|Default|GetHetch) (Math|Vector|Lerp(Vector) _startposition (- _startposition "0.000000,500.000000,0.000000") _speed) false false))))

(event EventBeginPlay
  (Variables|Default|SetStartPosition (Variables|/Script/Engine.SceneComponent|GetRelativeLocation (Variables|Default|GetHetch))))

(fn ConstructionScript)